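; Enemy actor with a Spine skeleton that reacts to hits with an animation and a sound.
; OnHit takes a name and a tick, using a map of the last tick per name to ignore repeat hits from the same name on the same tick.
; A new hit updates the map, plays the non-looping Hit animation and a 2D kill sound.
; The renderer's component hit event only prints debug text, and no health or death logic is present.
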(event `self.ReceiveBeginPlay`)

(event `self.SpineSkeletonRenderer.OnComponentHit`
  (params (HitComponent :type "PrimitiveComponent Object Reference") (OtherActor :type "Actor Object Reference") (OtherComp :type "PrimitiveComponent Object Reference") (NormalImpulse :type "Vector Structure") (Hit :type "HitResult Structure (by ref)"))
  (`KismetSystemLibrary.PrintString` "onHIT" true true (struct :`R` 1.0 :`G` 0.040289 :`B` 0.184118 :`A` 1.0)))

(event `OnHit`
  (params (Name :type String) (CurTick :type Integer64))
  (bind _newvar_0 (`self.NewVar_0`))
  (bind (_value _returnvalue) (`BlueprintMapLibrary.Map_Find` _newvar_0 Name))
  (if _returnvalue
    (if (not (== CurTick _value))
      (`BlueprintMapLibrary.Map_Add` _newvar_0 Name CurTick :!label _label)
      (`SpineSkeletonAnimationComponent.SetAnimation` (`self.SpineSkeletonAnimation`) 0 "Hit" false)
      (`GameplayStatics.PlaySound2D` "/Game/temp/kill_sound.kill_sound" 1.0 1.0 0.0 null null))
    (else
      (goto _label))))

(event `self.Box.OnComponentHit`
  (params (HitComponent :type "PrimitiveComponent Object Reference") (OtherActor :type "Actor Object Reference") (OtherComp :type "PrimitiveComponent Object Reference") (NormalImpulse :type "Vector Structure") (Hit :type "HitResult Structure (by ref)")))

(fn `UserConstructionScript`)