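; Base Blueprint for movable Spine-animated actors, providing shared animation playback and facing logic.
; PlayAnimation caches the current animation name and sets a track animation only when the name changes, so repeated calls do not restart it.
; MoveMentInput flips the Spine renderer by a 180-degree world rotation according to whether ScaleValue is above or below CompareWith.
; It applies no movement itself, leaving WorldDirection and Force unused.
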(event `PlayAnimation`
  (params (trackIndex :type Integer) (animationName :type String) (loop :type Boolean))
  ;[1 1 1] 播放动画
  (if (not (`KismetStringLibrary.EqualEqual_StrStr` (`self.CurAnimation`) animationName))
    (bind _output_get (set `self.CurAnimation` animationName))
    (`SpineSkeletonAnimationComponent.SetAnimation` (`self.SpineSkeletonAnimation`) trackIndex _output_get loop)))

(event `MoveMentInput`
  (params (WorldDirection :type "Vector Structure") (ScaleValue :type "Float (double-precision)") (bForce :type Boolean) (CompareWith :type "Float (double-precision)"))
  (bind _spineskeletonrenderer (`self.SpineSkeletonRenderer`))
  (`|ExecutionSequence`
    (:`then_1`
      (`/Engine/EditorBlueprintResources/StandardMacros.CompareFloat` ScaleValue CompareWith
        (:`>`
          (`SceneComponent.K2_SetWorldRotation` :`self` _spineskeletonrenderer))
        (:`<`
          (`SceneComponent.K2_SetWorldRotation` _spineskeletonrenderer (struct :`Yaw` 180.0) false false))))))

(fn `UserConstructionScript`)