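; Base character Blueprint with side-on movement that flips the animation manager's render rotation to face left or right.
; When an animation starts with a matching curve in CvRootLineList, a timeline fakes root motion by moving the capsule along X by the animation's RootDistance.
; Movement input locks during this motion until the curve value reaches RecoverTime or a short forward line trace from the child actor hits an obstacle.
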(event `self.ReceiveBeginPlay`
  (set `CharacterMovementComponent.MaxWalkSpeed` (`self.MaxSpeed`) (`self.CharacterMovement`))
  (bind _asbp_scanimation_manager (cast `/Game/Blueprint/GameBase/BP_SCAnimationManager` (`self.AnimationManager`)))
  (set `self.SCAnim` _asbp_scanimation_manager)
  (`self.CallBack`))

(event `self.ReceiveTick`
  (params (DeltaSeconds :type "Float (single-precision)")))

(event `MoveMentInput`
  (params (WorldDirection :type "Vector Structure") (ScaleValue :type "Float (double-precision)") (bForce :type Boolean) (CompareWith :type "Float (double-precision)") (IsMove :type Boolean))
  (bind _scanim (`self.SCAnim`))
  ;[1 1 1] 移动控制
  (`|ExecutionSequence`
    (:`then_0`
      (set `self.CanMove` IsMove)
      (if (`self.CanMove`)
        (`self.AddMovementInput` WorldDirection ScaleValue bForce)))
    (:`then_1`
      (if (`self.CanbeTurned`)
        (`/Engine/EditorBlueprintResources/StandardMacros.CompareFloat` ScaleValue CompareWith
          (:`>`
            (set `self.Direction` 1.0)
            (`/Game/Blueprint/GameBase/BP_SCAnimationManager.SetRenderRotation` :`self` _scanim))
          (:`<`
            (set `self.Direction` -1.0)
            (`/Game/Blueprint/GameBase/BP_SCAnimationManager.SetRenderRotation` _scanim (struct :`Yaw` 180.0))))))))

(event `AnimStart`
  (params (Anim :type "AnimationInfo Structure"))
  (bind (_value _returnvalue) (`BlueprintMapLibrary.Map_Find` (`self.CvRootLineList`) (`.AnimationName` (break `AnimationInfo` Anim))))
  ;[1 1 1] 回调处理
  (if _returnvalue
    (`self.RootLine` _value Anim)))

(event `CallBack`
  (bind _scanim (`self.SCAnim`))
  ;[1 1 1] 回调处理
  (`|ExecutionSequence`
    (:`then_0`
      (add `/Game/Blueprint/GameBase/BP_SCAnimationManager.OnAnimationStart` _scanim (delegate `AnimStart`)))
    (:`then_1`
      (add `/Game/Blueprint/GameBase/BP_SCAnimationManager.OnAnimationEnd` _scanim (delegate `AnimEnd`)))))

(event `AnimEnd`
  (params (Anim :type "AnimationInfo Structure"))
  ;[1 1 1] 回调处理
)

(event `RootLine`
  (params (Curve :type "CurveFloat Object Reference") (Anim :type "AnimationInfo Structure"))
  (bind (_name _animationname _trackindex _isplaying _isloop _rootdistance _recovertime) (break `AnimationInfo` Anim))
  (bind (_start_x _start_y _start_z) (`KismetMathLibrary.BreakVector` (`self.Start`)))
  ;[1 1 1] RootLine
  (if (`self.CanRootLine`)
    (set `self.in` true)
    (set `self.Start` (`SceneComponent.K2_GetComponentLocation` (`self.CapsuleComponent`)))
    (bind (_direction _time) (`Timeline|Timeline_0` :!via `PlayFromStart` :!label _label)
      (:`Update`
        (`|ExecutionSequence`
          (:`then_0`
            (`self.wwq`))
          (:`then_1`
            (set `self.CanMove` false)
            (bind _returnvalue (`CurveFloat.GetFloatValue` Curve _time))
            (`/Engine/EditorBlueprintResources/StandardMacros.CompareFloat` _returnvalue _recovertime
              (:`>`
                (`self.StopTL` :!label _label_2))
              (:`==`
                (goto _label_2))
              (:`<`
                (if (`self.in`)
                  (`SceneComponent.K2_SetWorldLocation` (`self.CapsuleComponent`) (`KismetMathLibrary.VLerp` (`self.Start`) (`KismetMathLibrary.MakeVector` (+ _start_x (* (`self.Direction`) _rootdistance)) _start_y _start_z) _returnvalue) false false)
                  (else
                    (goto _label_2)))))))))))

(event `StopTL`
  ;[1 1 1] RootLine
  (set `self.CanMove` true)
  (goto _label :!via `Stop`))

(event `wwq`
  (bind _returnvalue (`SceneComponent.K2_GetComponentLocation` (`self.ChildActor`)))
  ;[1 1 1] 碰撞检查
  (bind (_outhits _returnvalue_2) (`KismetSystemLibrary.LineTraceMulti` :`Start` _returnvalue :`End` (`KismetMathLibrary.MakeVector` (+ (.x _returnvalue) (* (`self.Direction`) 50.0)) (.y _returnvalue) (.z _returnvalue)) :`TraceChannel` "TraceTypeQuery1" :`TraceColor` (struct :`R` 0.101543 :`G` 0.372602 :`B` 1.0 :`A` 1.0)))
  (set `self.in` (not _returnvalue_2))
  (if _returnvalue_2
    (for _ _outhits
      _)))

(fn `EntryToAnim`
  (params (Entry :type "TrackEntry Object Reference"))
  (returns (IsFind :type Boolean) (Anim :type "AnimationInfo Structure"))
  (bind _animationinfolist (`self.AnimationInfoList`))
  (bind _returnvalue (`TrackEntry.getAnimationName` Entry))
  (bind _keys (`BlueprintMapLibrary.Map_Keys` _animationinfolist))
  (for _array_element _keys
    (bind _value (`BlueprintMapLibrary.Map_Find` _animationinfolist _array_element))
    (if (`KismetStringLibrary.EqualEqual_StrStr` (`.AnimationName` (break `AnimationInfo` _value)) _returnvalue)
      (return true _value)))
  (return false))

(fn `UserConstructionScript`)