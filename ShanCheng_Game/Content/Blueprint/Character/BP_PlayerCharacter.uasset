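; Player character Blueprint for single-axis melee combat with attack, tap-to-dodge/hold-to-sprint, jump and phased block.
; Animation data times each action's recovery and end, gating turning, movement and root-line flags before SCStateManager restores Idle.
; Attacks line-trace between weapon bones, passing the attack's tick to BP_Enemy.OnHit.
; Jumps raise the capsule along a timeline-driven curve, then poll IsFalling on a looping timer until landing.
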(event `self.ReceiveBeginPlay`
  (`parent.ReceiveBeginPlay`)
  (`self.Init`))

(event `self.ReceiveActorBeginOverlap`
  (params (OtherActor :type "Actor Object Reference"))
  (`parent.ReceiveActorBeginOverlap` OtherActor))

(event `self.ReceiveTick`
  (params (DeltaSeconds :type "Float (single-precision)"))
  (`parent.ReceiveTick` DeltaSeconds))

(event `Init`
  ;[1 1 1] 初始化
)

(event `InputAxis|MoveRigth`
  (params (AxisValue :type "Float (single-precision)"))
  ;[1 1 1] 移动
  (`|ExecutionSequence`
    (:`then_0`
      (if (`self.IsMove`)
        (`self.MoveMentInput` (`SceneComponent.GetRightVector` (`self.Camera`)) (* AxisValue (`self.scale`)) false 0.0 (not (`|EnumEquality` (`self.GetState`) "Attack")))))
    (:`then_1`
      (`/Engine/EditorBlueprintResources/StandardMacros.CompareFloat` (* AxisValue (`self.Direction`))
        (:`>`
          (set `self.IsForward` true :!label _label))
        (:`==`
          (goto _label))
        (:`<`
          (set `self.IsForward` false))))))

(event `self.AttackDetection`
  (params (_Name :type String))
  (bind _scanim (`self.SCAnim`))
  (bind _bonetransform_location (`KismetMathLibrary.BreakTransform` (`/Game/Blueprint/GameBase/BP_SCAnimationManager.GetBoneTransform` _scanim "wq_a")))
  (bind _bonetransform_location_2 (`KismetMathLibrary.BreakTransform` (`/Game/Blueprint/GameBase/BP_SCAnimationManager.GetBoneTransform` _scanim "wq_c")))
  ;[1 1 1] 攻击实质检查
  (bind _outhits (`KismetSystemLibrary.LineTraceMulti` :`Start` _bonetransform_location :`End` (`KismetMathLibrary.MakeVector` (+ (* (`self.Direction`) 15.0) (.x _bonetransform_location_2)) (.y _bonetransform_location_2) (.z _bonetransform_location_2)) :`TraceChannel` "TraceTypeQuery1" :`DrawDebugType` "ForOneFrame"))
  (for _array_element _outhits
    (bind _asbp_enemy (cast `/Game/Blueprint/Enemy/BP_Enemy` (`.HitActor` (`GameplayStatics.BreakHitResult` _array_element))))
    (`/Game/Blueprint/Enemy/BP_Enemy.OnHit` _asbp_enemy _Name (`self.CurTick`))))

(event `self.StartAttack_E`
  (params (Anim :type "AnimationInfo Structure"))
  ;[1 1 1] 攻击事件
  (set `self.CanbeTurned` false)
  (set `self.CanRootLine` true)
  (set `self.CurTick` (`SCBPFunction.GetCurTick`))
  (`KismetSystemLibrary.Delay` (`.RecoverTime` (break `AnimationInfo` Anim)))
  (set `self.CanRootLine` false)
  (`self.RevertAttack` Anim))

(event `EndUpDateT`
  ;[1 1 1] 攻击事件
  (`KismetSystemLibrary.K2_ClearAndInvalidateTimerHandle` (stale `self.RevertAttack_E` _returnvalue)))

(event `InputAction|SpeedUp`
  (params (Key :type "Key Structure"))
  ;[1 1 1] 加速
  (:`Pressed`
    (bind _returnvalue (`KismetSystemLibrary.K2_SetTimerDelegate` (delegate `CustomEvent_1`) 0.3)))
  (:`Released`
    (`KismetSystemLibrary.K2_ClearAndInvalidateTimerHandle` _returnvalue)
    (if (`self.IsSpeedUp`)
      (set `self.IsSpeedUp` false)
      (set `self.scale` (`self.SpeedConstraint`))
      (else
        (`self.Dodge`)))))

(event `self.RevertAttack_E`
  (params (Anim :type "AnimationInfo Structure"))
  ;[1 1 1] 攻击事件
  (bind _returnvalue (`KismetSystemLibrary.K2_SetTimerDelegate` (delegate `UpDtaeT`) (`.EndTime` (break `AnimationInfo` Anim)))))

(event `CustomEvent_1`
  ;[1 1 1] 加速
  (if (not (`self.IsSpeedUp`))
    (set `self.IsSpeedUp` true)
    (set `self.scale` 1.0)))

(event `UpDtaeT`
  ;[1 1 1] 攻击事件
  (`self.EndAttack` (stale `self.RevertAttack_E` Anim)))

(event `InputAction|Attack`
  (params (Key :type "Key Structure"))
  ;[1 1 1] 攻击
  (:`Pressed`
    (`self.Attack`)))

(event `self.EndAttack_E`
  (params (Anim :type "AnimationInfo Structure"))
  ;[1 1 1] 攻击事件
  (set `self.CanbeTurned` true)
  (`self.ResetAttackData`)
  (bind _returnvalue (`SCBPFunction.GetSCStateManager` self))
  (`SCStateManager.RestoreCharacterStateIdle` _returnvalue self "Attack"))

(event `self.StartDodge`
  (params (Anim :type "AnimationInfo Structure"))
  ;[1 1 1] 翻滚
  (set `self.CanbeTurned` false)
  (set `self.IsMove` false)
  (set `self.CanRootLine` true)
  (`KismetSystemLibrary.Delay` (`.RecoverTime` (break `AnimationInfo` Anim)))
  (set `self.CanRootLine` false)
  (set `self.CanbeTurned` true)
  (set `self.IsMove` true)
  (bind _returnvalue (`SCBPFunction.GetSCStateManager` self))
  (`SCStateManager.RestoreCharacterStateIdle` _returnvalue self "Dodge"))

(event `InputAction|Jump`
  (params (Key :type "Key Structure"))
  ;[1 1 1] 跳跃
  (:`Pressed`
    (`self.Jump_P`)))

(event `self.StartJump`
  (params (Anim :type "AnimationInfo Structure"))
  (bind (_name _animationname _trackindex _isplaying _isloop _rootdistance _recovertime _endtime) (break `AnimationInfo` Anim))
  ;[1 1 1] 跳跃事件
  (set `self.CanbeTurned` false)
  (`self.JumpLine` _endtime)
  (`KismetSystemLibrary.Delay` _endtime)
  (`self.Loop`))

(event `JumpLine`
  (params (EndTime :type "Float (double-precision)"))
  (bind _capsulecomponent (`self.CapsuleComponent`))
  (bind (_startj_x _startj_y _startj_z) (`KismetMathLibrary.BreakVector` (`self.StartJ`)))
  (bind (_returnvalue_x _returnvalue_y) (`KismetMathLibrary.BreakVector` (`SceneComponent.K2_GetComponentLocation` _capsulecomponent)))
  ;[1 1 1] 起跳
  (set `self.StartJ` (`SceneComponent.K2_GetComponentLocation` (`self.CapsuleComponent`)))
  (bind (_direction _time) (`Timeline|Timeline_1_0` :!via `PlayFromStart` :!label _label_2)
    (:`Update`
      (if (> _time EndTime)
        (goto _label_2 :!via `Stop`)
        (else
          (`SceneComponent.K2_SetWorldLocation` _capsulecomponent (`KismetMathLibrary.MakeVector` _returnvalue_x _returnvalue_y (+ _startj_z (* (`CurveFloat.GetFloatValue` (`self.Cv_StartJump`) _time) 150.0))) false false))))))

(event `self.LoopJump`
  (params (Anim :type "AnimationInfo Structure"))
  ;[1 1 1] 跳跃事件
  (`KismetSystemLibrary.Delay` 0.2)
  (`self.JumpAfter` (`NavMovementComponent.IsFalling` (`self.CharacterMovement`))))

(event `EndLoop`
  ;[1 1 1] 空中循环
  (`KismetSystemLibrary.K2_ClearAndInvalidateTimerHandle` (stale `Loop` _returnvalue)))

(event `Loop`
  ;[1 1 1] 空中循环
  (`self.JumpAfter` (`NavMovementComponent.IsFalling` (`self.CharacterMovement`)))
  (bind _returnvalue (`KismetSystemLibrary.K2_SetTimerDelegate` (delegate `CustomEvent_0`) 0.01 true)))

(event `self.EndJump`
  (params (Anim :type "AnimationInfo Structure"))
  ;[1 1 1] 跳跃事件
  (set `self.IsMove` false)
  (`self.EndLoop`)
  (`KismetSystemLibrary.Delay` (`.EndTime` (break `AnimationInfo` Anim)))
  (set `self.IsMove` true)
  (set `self.IsJump` false)
  (set `self.CanbeTurned` true)
  (`self.ResetAttackData`)
  (bind _returnvalue (`SCBPFunction.GetSCStateManager` self))
  (`SCStateManager.RestoreCharacterStateIdle` _returnvalue self "Jump"))

(event `CustomEvent_0`
  ;[1 1 1] 空中循环
  (`self.JumpAfter` (`NavMovementComponent.IsFalling` (`self.CharacterMovement`))))

(event `Key|One`
  (params (Key :type "Key Structure"))
  ;[1 1 1] Comment
  (:`Pressed`
    (set `self.IsHit` true)
    (set `self.IsMove` false))
  (:`Released`
    (set `self.IsHit` false)
    (set `self.IsMove` true)))

(event `InputAxis|Defense`
  (params (AxisValue :type "Float (single-precision)"))
  (bind _returnvalue (== AxisValue 0.0))
  ;[1 1 1] 格挡
  (`|ExecutionSequence`
    (:`then_0`
      (if (not _returnvalue)
        (`|ExecutionSequence`
          (:`then_0`
            (set `self.CanbeTurned` false)
            (set `self.scale` 0.2)
            (`self.Defense`))
          (:`then_1`
            (`/Engine/EditorBlueprintResources/StandardMacros.DoOnce` false :!label _label_3
              (:`Completed`
                (set `self.DefensePhase` 1)
                (`KismetSystemLibrary.Delay` 0.3)
                (set `self.DefensePhase` 2)))))
        (else
          (`/Engine/EditorBlueprintResources/StandardMacros.DoOnce` false :!label _label_4
            (:`Completed`
              (set `self.CanbeTurned` true)
              (set `self.scale` (`self.SpeedConstraint`))
              (set `self.IsDefense` false)
              (set `self.DefensePhase` 0)
              (bind _returnvalue_2 (`SCBPFunction.GetSCStateManager` self))
              (`SCStateManager.RestoreCharacterStateIdle` _returnvalue_2 self "Defense"))))))
    (:`then_1`
      (if _returnvalue
        (goto _label_3 :!via `Reset`)
        (else
          (goto _label_4 :!via `Reset`))))))

(fn `UserConstructionScript`)