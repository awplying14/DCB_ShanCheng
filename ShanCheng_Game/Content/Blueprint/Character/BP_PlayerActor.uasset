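; BP_PlayerActor is the player character Blueprint, driving track-based locomotion animation and registering a three-step attack combo.
; On BeginPlay, it fills attack lookup maps through SetAttackInfo, then starts a looping timer, which StopUpdate can clear.
; Instead of Tick, the timer selects idle, jog or run from velocity while IsRemovable is set.
; The movement axis handler is an empty stub, and nothing here plays the attacks.
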(event `Init`
  (`|ExecutionSequence`
    (:`then_0`
      (`self.SetAttackInfo` 0 "Attack1_1")
      (`self.SetAttackInfo` 1 "Attack1_2")
      (`self.SetAttackInfo` 2 "Attack1_3"))
    (:`then_1`
      (`self.StartUpdate`))))

(event `StopUpdate`
  ;[1 1 1] 更新动画
  (`KismetSystemLibrary.K2_ClearAndInvalidateTimerHandle` (stale `StartUpdate` _returnvalue)))

(event `self.ReceiveBeginPlay`
  (`self.Init`))

(event `StartUpdate`
  ;[1 1 1] 更新动画
  (bind _returnvalue (`KismetSystemLibrary.K2_SetTimerDelegate` (delegate `UPdateAnimaton`) 0.1 true)))

(event `InputAxis|MoveRigth`
  (params (AxisValue :type "Float (single-precision)"))
  ;[1 1 1] 移动
  (if (`self.IsRemovable`)
    _))

(event `UPdateAnimaton`
  (bind _returnvalue (`KismetMathLibrary.VSize` (`self.GetVelocity`)))
  ;[1 1 1] 更新动画
  (if (`self.IsRemovable`)
    (`/Engine/EditorBlueprintResources/StandardMacros.CompareFloat` _returnvalue
      (:`>`
        (`/Engine/EditorBlueprintResources/StandardMacros.CompareFloat` _returnvalue 245.0
          (:`>`
            (`self.PlayAnimation` 0 "Run"))
          (:`==`
            (`self.PlayAnimation` 0 "Jog" :!label _label))
          (:`<`
            (goto _label))))
      (:`==`
        (`self.PlayAnimation` 0 "Idle1" :!label _label_2))
      (:`<`
        (goto _label_2)))))

(fn `SetAttackInfo`
  (params (Key :type Integer) (AnimationName :type String) (TrackIndex :type Integer) (IsLoop :type Boolean))
  (`BlueprintMapLibrary.Map_Add` (`self.AttackList`) Key AnimationName)
  (`BlueprintMapLibrary.Map_Add` (`self.AttackInfoList`) AnimationName (make `/Game/Blueprint/ST/ST_AttackInfo` AnimationName TrackIndex IsLoop)))

(fn `UserConstructionScript`)