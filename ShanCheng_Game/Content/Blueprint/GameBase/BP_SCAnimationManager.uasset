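; Base-style actor that manages Spine skeletal animation, with helpers for render rotation and bone transforms.
; PlayAnimationEvent starts animations not already playing and tracks their state in a name-keyed map.
; Spine start/end events map track entries back to that map, update state, relay callbacks and print debug text.
; On start, a Timeline polls notify trigger times to fire OnAnimNotity until EndTime, restarting for playing loops.
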(event `self.ReceiveBeginPlay`
  (`self.Init`))

(event `Init`)

(event `SetRenderRotation`
  (params (Rotation :type "Rotator Structure"))
  ;[1 1 1] Comment
  (`SceneComponent.K2_SetWorldRotation` (`self.SpineSkeletonRenderer`) Rotation false false))

(event `self.PlayAnimationEvent`
  (params (Anim :type "AnimationInfo Structure"))
  (bind (_name _animationname _trackindex _isplaying _isloop) (break `AnimationInfo` Anim))
  ;[1 1 1] 播放动画
  (if (not _isplaying)
    (set `self.CurAnimation` _animationname)
    (`SpineSkeletonAnimationComponent.SetAnimation` (`self.SpineSkeletonAnimation`) _trackindex _animationname _isloop)
    (bind _structout (setmembers `AnimationInfo` :`StructRef` Anim :`IsPlaying` true))
    (`BlueprintMapLibrary.Map_Add` (`self.AnimationInfoList`) _name _structout)))

(event `AnimNotityListening`
  (params (Anim :type "AnimationInfo Structure"))
  (bind (_name _animationname _trackindex _isplaying _isloop _rootdistance _recovertime _endtime _notyflist) (break `AnimationInfo` Anim))
  ;[1 1 1] 监听动画通知
  (`self.InitAnimNotify`)
  (if (!= (`KismetArrayLibrary.Array_Length` _notyflist) 0)
    (bind (_direction _time) (`Timeline|Timeline_0` :!via `PlayFromStart` :!label _label)
      (:`Update`
        (`/Engine/EditorBlueprintResources/StandardMacros.CompareFloat` _time _endtime
          (:`>`
            (`self.EndAnimNotityListening` :!label _label_2))
          (:`==`
            (goto _label_2))
          (:`<`
            (for (_array_element _array_index) _notyflist
              (`/Engine/EditorBlueprintResources/StandardMacros.CompareFloat` _time (`.TriggerTime` (break `SpineAnimNotify` _array_element))
                (:`>`
                  (`self.OnAnimNotity` _array_element _array_index))))))))))

(event `EndAnimNotityListening`
  ;[1 1 1] 监听动画通知
  (`|ExecutionSequence`
    (:`then_0`
      (goto _label :!via `Stop`))
    (:`then_1`
      (bind (_name _animationname _trackindex _isplaying _isloop _rootdistance _recovertime _endtime _notyflist) (break `AnimationInfo` (stale `AnimNotityListening` Anim)))
      (if (and _isloop _isplaying)
        (`self.AnimNotityListening` (stale `AnimNotityListening` Anim))))))

(event `self.SpineSkeletonAnimation.AnimationStart`
  (params (entry :type "TrackEntry Object Reference"))
  ;[1 1 1] 动画开始
  (`|ExecutionSequence`
    (:`then_0`
      (bind (_isfind _anim) (`self.EntryToAnim` entry))
      (if _isfind
        (`|ExecutionSequence`
          (:`then_0`
            (`self.AnimNotityListening` _anim))
          (:`then_1`
            (`self.OnAnimationStart` _anim)))))
    (:`then_1`
      (bind _returnvalue (`TrackEntry.getAnimationName` entry))
      (bind _returnvalue_2 (`TrackEntry.GetAnimationEnd` entry))
      (`KismetSystemLibrary.PrintString` (`KismetTextLibrary.Conv_TextToString` (`|FormatText` "{n}----{s}" _returnvalue _returnvalue_2)) true false (struct :`G` 0.66 :`B` 1.0 :`A` 1.0) 20.0))))

(event `self.SpineSkeletonAnimation.AnimationEnd`
  (params (entry :type "TrackEntry Object Reference"))
  ;[1 1 1] 动画结束
  (`|ExecutionSequence`
    (:`then_0`
      (bind (_isfind _anim) (`self.EntryToAnim` entry))
      (if _isfind
        (`|ExecutionSequence`
          (:`then_0`
            (bind _structout (setmembers `AnimationInfo` :`StructRef` _anim :`IsPlaying` false))
            (`BlueprintMapLibrary.Map_Add` (`self.AnimationInfoList`) (`.Name` (break `AnimationInfo` _anim)) _structout))
          (:`then_1`
            (`self.OnAnimationEnd` _anim)))))
    (:`then_1`
      (bind _returnvalue (`TrackEntry.getAnimationName` entry))
      (bind _returnvalue_2 (`TrackEntry.GetAnimationEnd` entry))
      (`KismetSystemLibrary.PrintString` (`KismetTextLibrary.Conv_TextToString` (`|FormatText` "{n}----{s}" _returnvalue _returnvalue_2)) true false (struct :`R` 1.0 :`G` 0.008175 :`B` 0.071885 :`A` 1.0) 20.0))))

(fn `EntryToAnim`
  (params (Entry :type "TrackEntry Object Reference"))
  (returns (IsFind :type Boolean) (Anim :type "AnimationInfo Structure"))
  (bind _animationinfolist (`self.AnimationInfoList`))
  (bind _returnvalue (`TrackEntry.getAnimationName` Entry))
  (bind _keys (`BlueprintMapLibrary.Map_Keys` _animationinfolist))
  (for _array_element _keys
    (bind _value (`BlueprintMapLibrary.Map_Find` _animationinfolist _array_element))
    (if (`KismetStringLibrary.EqualEqual_StrStr` (`.AnimationName` (break `AnimationInfo` _value)) _returnvalue)
      (return true _value)))
  (return false))

(fn `GetBoneTransform`
  (params (BoneName :type String))
  (returns (BoneTransform :type "Transform Structure"))
  (bind _returnvalue (`SpineSkeletonComponent.GetBoneWorldTransform` (`self.SpineSkeletonAnimation`) BoneName))
  (return _returnvalue))

(fn `UserConstructionScript`)