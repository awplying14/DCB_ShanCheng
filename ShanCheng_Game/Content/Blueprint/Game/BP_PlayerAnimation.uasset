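; Player animation Blueprint for a Spine character that registers its animation set and plays surface-dependent footsteps.
; Init registers locomotion, attack, jump, defense and dodge clips with loop, timing and root-distance settings, then adds left/right foot notifies to Jog and Run.
; Each notify prints its name and traces down from a foot bone, playing the footstep sound stored on any hit PM_SCEnvironment physical material.
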(event `self.Init`
  ;[1 1 1] 动画初始化
  (`|ExecutionSequence`
    (:`then_0`
      (`self.addAnimationToList` "Idle" "Idle1" 0 true 0.0 0.0 0.9)
      (`self.addAnimationToList` "Jog" "Jog" 0 true 0.0 0.0 0.9)
      (`self.addAnimationToList` "Run" "Run" 0 true 0.0 0.0 0.633)
      (`self.addAnimationToList` "Attack1" "Attack1_1" 0 false 80.0 0.5 0.34)
      (`self.addAnimationToList` "Attack2" "Attack1_2" 0 false 50.0 0.4 0.467)
      (`self.addAnimationToList` "Attack3" "Attack1_3" 0 false 50.0 0.6 0.267)
      (`self.addAnimationToList` "block3" "z_block3" 0 true))
    (:`then_1`
      (`self.addAnimationToList` "StartJump" "Jump_Start" 0 true 0.0 0.0 0.5)
      (`self.addAnimationToList` "LoopJump" "Jump_Loop" 0 true)
      (`self.addAnimationToList` "EndJump" "Jump_End" 0 false 0.0 0.0 0.267)
      (`self.addAnimationToList` "DefenseHit" "defense_Hit" 0 false 0.0 0.0 0.267)
      (`self.addAnimationToList` "DefenseIdle" "defense_Idle" 0 true)
      (`self.addAnimationToList` "DefenseForward" "defense_Jog_Forward" 0 true)
      (`self.addAnimationToList` "DefenseBackward" "defense_Jog_Backward" 0 true)
      (`self.addAnimationToList` "DodgeForward" "Dodge_Forward" 0 false 600.0 0.667)
      (`self.addAnimationToList` "DodgeBackward" "Dodge_Backward" 0 false -450.0 0.467))
    (:`then_2`
      (`self.SetNotityToAnimation` "Jog" (make `SpineAnimNotify` "Lefe" 0.2))
      (`self.SetNotityToAnimation` "Jog" (make `SpineAnimNotify` "Right" 0.66))
      (`self.SetNotityToAnimation` "Run" (make `SpineAnimNotify` "Lefe" 0.1))
      (`self.SetNotityToAnimation` "Run" (make `SpineAnimNotify` "Right" 0.43)))))

(event `self.ReceiveTick`
  (params (DeltaSeconds :type "Float (single-precision)"))
  (`parent.ReceiveTick` DeltaSeconds))

(event `self.OnAnimNotityEvent`
  (params (AnimNotify :type "SpineAnimNotify Structure"))
  ;[1 1 1] 动画通知
  (`self.Foot` AnimNotify))

(event `Foot`
  (params (SpineAnimNotify :type "SpineAnimNotify Structure (by ref)"))
  (bind _notifyname (break `SpineAnimNotify` SpineAnimNotify))
  (bind _bonetransform_location (`KismetMathLibrary.BreakTransform` (`self.GetBoneTransform` "zj_3")))
  (bind _bonetransform_location_2 (`KismetMathLibrary.BreakTransform` (`self.GetBoneTransform` "yj_3")))
  ;[1 1 1] 脚步声
  (`KismetSystemLibrary.PrintString` _notifyname true true (struct :`R` 0.092793 :`G` 1.0 :`B` 0.156864 :`A` 1.0) 1.0)
  (switch `string` _notifyname
    (:`Lefe`
      (`self.PlayFootStep` _bonetransform_location_2))
    (:`Right`
      (`self.PlayFootStep` _bonetransform_location))))

(event `PlayFootStep`
  (params (Location :type "Vector Structure"))
  ;[1 1 1] 检查地板材质来播放脚步声
  (bind _outhits (`KismetSystemLibrary.LineTraceMulti` :`Start` Location :`End` (`KismetMathLibrary.MakeVector` (.x Location) (.y Location) (+ (.z Location) -91.0)) :`TraceChannel` "TraceTypeQuery1" :`TraceColor` (struct :`R` 0.072937 :`G` 1.0 :`B` 0.035516 :`A` 1.0)))
  (for _array_element _outhits
    (bind _aspm_scenvironment (cast `PM_SCEnvironment` (`.PhysMat` (`GameplayStatics.BreakHitResult` _array_element))))
    (`GameplayStatics.PlaySoundAtLocation` (`PM_SCEnvironment.FootstepSound` _aspm_scenvironment) Location (struct) 1.0 1.0 0.0 null null null)))

(fn `UserConstructionScript`
  (`parent.UserConstructionScript`))